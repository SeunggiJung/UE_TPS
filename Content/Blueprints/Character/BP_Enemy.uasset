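; BP_Enemy is an enemy character Blueprint that can visually dissolve its mesh and keeps a link to its spawn point.
; BeginPlay replaces every mesh material with a dynamic instance and caches them in Materials.
; StartDissolve plays a timeline from the start, writing its curve value to the "Dissolve" scalar parameter on each cached material.
; LinkSpawnPoint only stores the given point in SpawnPoint.
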(event `self.ReceiveBeginPlay`
  (for (_array_element _array_index) (`MeshComponent.GetMaterials` (`self.Mesh`))
    (bind _returnvalue (`KismetMaterialLibrary.CreateDynamicMaterialInstance` _array_element))
    (`PrimitiveComponent.SetMaterial` (`self.Mesh`) _array_index _returnvalue)
    (`KismetArrayLibrary.Array_Add` (`self.Materials`) _returnvalue)))

(event `StartDissolve`
  (bind (_direction _dissolve) (`Timeline|타임라인(Dissolve)` :!via `PlayFromStart`)
    (:`Update`
      (for _array_element (`self.Materials`)
        (`MaterialInstanceDynamic.SetScalarParameterValue` _array_element "Dissolve" _dissolve)))))

(fn `LinkSpawnPoint`
  (params (Point :type "/Game/Blueprints/Character/BP_EnemySpawnPoint Object Reference"))
  (set `self.SpawnPoint` Point))

(fn `UserConstructionScript`)