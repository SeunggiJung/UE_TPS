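; Player controller that turns Enhanced Input actions into camera look, movement and jumping for the controlled pawn.
; BeginPlay adds IMC_Default to the local player's input subsystem, and IA_Look feeds yaw and pitch input.
; IA_Move rotates its input by control-rotation yaw for camera-relative movement, while IA_Jump casts the pawn to BP_character and calls Jump.
; An unrotated world-direction move and debug prints remain as disconnected nodes.
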(event `EnhancedInput|/Game/Blueprints/Inputs/IA_Move`
  (params (ActionValue :type "Vector Structure") (ElapsedSeconds :type "Float (double-precision)") (TriggeredSeconds :type "Float (double-precision)") (InputAction :type "InputAction Object Reference" :default "/Game/Blueprints/Inputs/IA_Move.IA_Move")))

(event `self.ReceiveBeginPlay`
  (`EnhancedInputSubsystemInterface.AddMappingContext` (subsystem `EnhancedInputLocalPlayerSubsystem`) "/Game/Blueprints/Inputs/IMC_Default.IMC_Default" 0 (struct)))

(event `EnhancedInput|/Game/Blueprints/Inputs/IA_Look`
  (params (ActionValue :type "Vector Structure") (ElapsedSeconds :type "Float (double-precision)") (TriggeredSeconds :type "Float (double-precision)") (InputAction :type "InputAction Object Reference" :default "/Game/Blueprints/Inputs/IA_Look.IA_Look"))
  ; 카메라 회전
  (:`Triggered`
    (`self.AddYawInput` ActionValue_X)
    (`self.AddPitchInput` ActionValue_Y)))

(event `EnhancedInput|/Game/Blueprints/Inputs/IA_Move`
  (params (ActionValue :type "Vector Structure") (ElapsedSeconds :type "Float (double-precision)") (TriggeredSeconds :type "Float (double-precision)") (InputAction :type "InputAction Object Reference" :default "/Game/Blueprints/Inputs/IA_Move.IA_Move"))
  ; 월드 방향 이동
)

(event `EnhancedInput|/Game/Blueprints/Inputs/IA_Move`
  (params (ActionValue :type "Vector Structure") (ElapsedSeconds :type "Float (double-precision)") (TriggeredSeconds :type "Float (double-precision)") (InputAction :type "InputAction Object Reference" :default "/Game/Blueprints/Inputs/IA_Move.IA_Move"))
  (bind (_returnvalue_roll _returnvalue_pitch _returnvalue_yaw) (`KismetMathLibrary.BreakRotator` (`self.GetControlRotation`)))
  ; 로컬 축 이동
  (:`Triggered`
    (`Pawn.AddMovementInput` (`self.K2_GetPawn`) (`KismetMathLibrary.GreaterGreater_VectorRotator` ActionValue (`KismetMathLibrary.MakeRotator` 0.0 0.0 _returnvalue_yaw)) 1.0 false)))

(event `EnhancedInput|/Game/Blueprints/Inputs/IA_Jump`
  (params (ActionValue :type Boolean) (ElapsedSeconds :type "Float (double-precision)") (TriggeredSeconds :type "Float (double-precision)") (InputAction :type "InputAction Object Reference" :default "/Game/Blueprints/Inputs/IA_Jump.IA_Jump"))
  ; 점프
  (:`Started`
    (bind _asbp_character (cast `/Game/Blueprints/Character/BP_character` (`self.K2_GetPawn`)))
    (`Character.Jump` _asbp_character)))

(fn `UserConstructionScript`)