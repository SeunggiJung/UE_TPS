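; BP_EnemySpawnPoint is a spawn point actor that keeps at most one BP_Enemy linked to it and schedules respawns.
; BeginPlay starts a delay timer, and OnSpawnEnemy spawns an enemy at the actor's location if none is valid.
; The spawned enemy receives a back-reference through LinkSpawnPoint.
; UnLinkEnemy clears the stored enemy, resets the delay to a fixed value and restarts the timer.
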(event `self.ReceiveBeginPlay`
  (`KismetSystemLibrary.K2_SetTimerDelegate` (`|CreateDelegate` :!event `OnSpawnEnemy`) (`self.SpawnDelayTime`)))

(fn `OnSpawnEnemy`
  (if (not (`KismetSystemLibrary.IsValid` (`self.SpawnEnemy`)))
    (bind _returnvalue (`|SpawnActorFromClass` "/Game/Blueprints/Character/BP_Enemy.BP_Enemy_C" (`KismetMathLibrary.MakeTransform` (`self.K2_GetActorLocation`)) "Undefined" "MultiplyWithRoot" null null))
    (bind _output_get (set `self.SpawnEnemy` _returnvalue))
    (`/Game/Blueprints/Character/BP_Enemy.LinkSpawnPoint` _output_get self)))

(fn `UnLinkEnemy`
  (params (Enemy :type "/Game/Blueprints/Character/BP_Enemy Object Reference"))
  (set `self.SpawnEnemy` null)
  (set `self.SpawnDelayTime` 5.0)
  (`KismetSystemLibrary.K2_SetTimerDelegate` (`|CreateDelegate` :!event `OnSpawnEnemy`) (`self.SpawnDelayTime`)))

(fn `UserConstructionScript`)