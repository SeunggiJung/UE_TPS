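; Enemy AI component that runs BP_Enemy as an Idle, Move, Attack, Damage and Die state machine on Tick.
; Move chases the player when near and path-reachable, otherwise patrols to a random navmesh point; Attack only prints and triggers animation.
; OnDamageProcess rolls random damage with critical chance, switches to Damage or Die, and broadcasts through BP_GameInstance's dispatcher.
; States sync to ABP_Enemy; dead enemies sink, unlink from their spawn point and are destroyed.
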(event `self.ReceiveBeginPlay`
  (`|ExecutionSequence`
    (:`then_0`
      (bind _returnvalue (`GameplayStatics.GetActorOfClass` "/Game/Blueprints/Character/BP_character.BP_character_C"))
      (set `self.TargetPlayer` _returnvalue)
      (bind _asbp_enemy (cast `/Game/Blueprints/Character/BP_Enemy` (`self.GetOwner`)))
      (set `self.Owner` _asbp_enemy))
    (:`then_1`
      (bind _asabp_enemy (cast `/Game/Blueprints/Character/ABP_Enemy` (`SkeletalMeshComponent.GetAnimInstance` (`Character.Mesh` (`self.Owner`)))))
      (set `self.Anim` _asabp_enemy))
    (:`then_2`
      (set `self.Ai` (`AIBlueprintHelperLibrary.GetAIController` (`self.Owner`))))))

(event `self.ReceiveTick`
  (params (DeltaSeconds :type "Float (single-precision)"))
  (`|ExecutionSequence`
    (:`then_0`
      (set `self.DeltaSeconds` DeltaSeconds))
    (:`then_1`
      (switch `/Game/Blueprints/Character/E_EnemyStates` (`self.State`)
        (:`NewEnumerator0`
          (`self.IdleState`))
        (:`NewEnumerator1`
          (`self.MoveState`))
        (:`NewEnumerator2`
          (`self.AttackState`))
        (:`NewEnumerator3`
          (`self.DamageState`))
        (:`NewEnumerator4`
          (`self.DieState`))))))

(fn `AssignTarget`
  (bind _asabp_enemy (cast `/Game/Blueprints/Character/ABP_Enemy` (`SkeletalMeshComponent.GetAnimInstance` (`Character.Mesh` (`self.Owner`)))))
  (set `/Game/Blueprints/Character/ABP_Enemy.TargetPlayer` (`self.TargetPlayer`) _asabp_enemy))

(fn `AttackState`
  (bind _output_get (set `self.CurrentTime` (+ (`self.CurrentTime`) (`self.DeltaSeconds`))))
  (if (> _output_get (`self.AttackDelayTime`))
    (`KismetSystemLibrary.PrintString` "Attack!!! \n")
    (set `self.CurrentTime` 0.0)
    (set `/Game/Blueprints/Character/ABP_Enemy.bAttackPlay` true (`self.Anim`))
    (elif (> (`KismetMathLibrary.Vector_Distance` (`Actor.K2_GetActorLocation` (`self.TargetPlayer`)) (`Actor.K2_GetActorLocation` (`self.Owner`))) (`self.AttackOutRange`))
      (bind _output_get_2 (set `self.State` "NewEnumerator0"))
      (set `self.CurrentTime` 0.0)
      (set `/Game/Blueprints/Character/ABP_Enemy.AnimState` _output_get_2 (`self.Anim`)))))

(fn `CriticalCheck`
  (if (< (`KismetMathLibrary.RandomIntegerInRange` 0 100) 20)
    (set `self.bIsCritical` true)
    (set `self.DamageValue` (`KismetMathLibrary.Conv_IntToDouble` (`KismetMathLibrary.RandomIntegerInRange` 200 300)))
    (else
      (set `self.bIsCritical` false)
      (set `self.DamageValue` (`KismetMathLibrary.Conv_IntToDouble` (`KismetMathLibrary.RandomIntegerInRange` 100 200))))))

(fn `DamageState`
  (bind _output_get (set `self.CurrentTime` (+ (`self.CurrentTime`) (`self.DeltaSeconds`))))
  (if (> _output_get (`self.DamageDelayTime`))
    (bind _output_get_2 (set `self.State` "NewEnumerator0"))
    (set `self.CurrentTime` 0.0)
    (set `/Game/Blueprints/Character/ABP_Enemy.AnimState` _output_get_2 (`self.Anim`))))

(fn `DieState`
  (bind (_diepos_x _diepos_y _diepos_z) (`KismetMathLibrary.BreakVector` (`self.DiePos`)))
  (bind _owner (`self.Owner`))
  (bind (_enemydiepos_x _enemydiepos_y _enemydiepos_z) (`KismetMathLibrary.BreakVector` (`self.EnemyDiePos`)))
  (if (`/Game/Blueprints/Character/ABP_Enemy.bDieDone` (`self.Anim`))
    (`|ExecutionSequence`
      (:`then_0`
        (bind _output_get (set `self.DiePos` (+ (`Actor.K2_GetActorLocation` (`self.Owner`)) (* (`KismetMathLibrary.Vector_Down`) (`self.DieSpeed`) (`self.DeltaSeconds`)))))
        (`Actor.K2_SetActorLocation` (`self.Owner`) _output_get false false))
      (:`then_1`
        (if (<= _diepos_z (+ _enemydiepos_z -200.0))
          (`/Game/Blueprints/Character/BP_EnemySpawnPoint.UnLinkEnemy` (`/Game/Blueprints/Character/BP_Enemy.SpawnPoint` _owner) null)
          (`Actor.K2_DestroyActor` _owner))))))

(fn `FindPathTargetLocation`
  (returns (Result :type Boolean))
  (bind _returnvalue (`NavigationSystemV1.FindPathToLocationSynchronously` (`Actor.K2_GetActorLocation` (`self.Owner`)) (`Actor.K2_GetActorLocation` (`self.TargetPlayer`)) (`self.Ai`) null))
  (return (`NavigationPath.IsValid` _returnvalue)))

(fn `GetRandomPositionInNavMesh`
  (params (CenterLocation :type "Vector Structure") (Radius :type "Float (double-precision)"))
  (returns (Dest :type "Vector Structure") (bResult :type Boolean))
  (bind (_randomlocation _returnvalue) (`NavigationSystemV1.K2_GetRandomReachablePointInRadius` CenterLocation Radius null null))
  (return _randomlocation _returnvalue))

(fn `GetTargetDistance`
  (returns (Return :type "Float (double-precision)"))
  (return (`KismetMathLibrary.Vector_Distance` (`Actor.K2_GetActorLocation` (`self.TargetPlayer`)) (`Actor.K2_GetActorLocation` (`self.Owner`)))))

(fn `IdleState`
  (locals (RandomPosRadius :type "Float (double-precision)" :default 700.0))
  (bind _output_get (set `self.CurrentTime` (+ (`self.CurrentTime`) (`self.DeltaSeconds`))))
  (if (> _output_get (`self.IdleDelayTime`))
    (`|ExecutionSequence`
      (:`then_0`
        (bind _output_get_2 (set `self.State` "NewEnumerator1"))
        (set `self.CurrentTime` 0.0)
        (`self.AssignTarget`))
      (:`then_1`
        (set `/Game/Blueprints/Character/ABP_Enemy.AnimState` _output_get_2 (`self.Anim`)))
      (:`then_2`
        (bind _dest (`self.GetRandomPositionInNavMesh` (`Actor.K2_GetActorLocation` (`self.Owner`)) (`local.RandomPosRadius`)))
        (set `self.RandomPos` _dest)))))

(fn `MoveState`
  (bind _return (`self.GetTargetDistance`))
  (if (< _return (`self.FindPathDistance`))
    (bind _result (`self.FindPathTargetLocation`))
    (if _result
      (`self.TargetMove`)
      (else
        (`self.PatrolMove`)))
    (else
      (`self.PatrolMove`))))

(fn `OnDamageProcess`
  (if (`|EnumInequality` (`self.State`) "NewEnumerator4")
    (set `self.DamageValue` (`KismetMathLibrary.Conv_IntToDouble` (`KismetMathLibrary.RandomIntegerInRange` 100 200)))
    (`|ExecutionSequence`
      (:`then_0`
        (`self.CriticalCheck`)
        (bind _output_get (set `self.Hp` (- (`self.Hp`) (`self.DamageValue`))))
        (if (<= _output_get 0)
          (bind _output_get_2 (set `self.State` "NewEnumerator4"))
          (`PrimitiveComponent.SetCollisionEnabled` (`Character.CapsuleComponent` (`self.Owner`)) "NoCollision")
          (set `/Game/Blueprints/Character/ABP_Enemy.AnimState` _output_get_2 (`self.Anim`))
          (`Character.PlayAnimMontage` (`self.Owner`) "/Game/Animations/EnemyDamageMontage.EnemyDamageMontage" 1.0 "Die")
          (set `self.EnemyDiePos` (`Actor.K2_GetActorLocation` (`self.Owner`)))
          (else
            (bind _output_get_3 (set `self.State` "NewEnumerator3"))
            (set `/Game/Blueprints/Character/ABP_Enemy.AnimState` _output_get_3 (`self.Anim`))
            (`/Game/Blueprints/Character/ABP_Enemy.PlayDamageAnim` (`self.Anim`) (`KismetStringLibrary.Conv_StringToName` (`KismetStringLibrary.Concat_StrStr` "Damage" (`KismetStringLibrary.Conv_IntToString` (`KismetMathLibrary.RandomIntegerInRange` 0 1))))))))
      (:`then_1`
        (bind _asbp_game_instance (cast `/Game/Blueprints/GameConfig/BP_GameInstance` (`GameplayStatics.GetGameInstance`)))
        (`/Game/Blueprints/GameConfig/BP_GameEventDispather.OnEnemyDamaged` (`/Game/Blueprints/GameConfig/BP_GameInstance.GameEventDispatcher` _asbp_game_instance) (`self.Owner`) (`self.DamageValue`) (`self.bIsCritical`))))))

(fn `PatrolMove`
  (bind _returnvalue (`AIController.MoveToLocation` (`self.Ai`) (`self.RandomPos`) -1.0 true true false true null true))
  (if (`|EnumEquality` _returnvalue "AlreadyAtGoal")
    (set `self.State` "NewEnumerator0")
    (set `self.CurrentTime` 0.0)
    (set `/Game/Blueprints/Character/ABP_Enemy.AnimState` "NewEnumerator0" (`self.Anim`))))

(fn `TargetMove`
  (bind _anim (`self.Anim`))
  (set `self.Dir` (- (`Actor.K2_GetActorLocation` (`self.TargetPlayer`)) (`Actor.K2_GetActorLocation` (`self.Owner`))))
  (`AIController.MoveToLocation` (`self.Ai`) (`Actor.K2_GetActorLocation` (`self.TargetPlayer`)) -1.0 true true false true null true)
  (if (< (`KismetMathLibrary.VSize` (`self.Dir`)) (`self.AttackRange`))
    (`|ExecutionSequence`
      (:`then_0`
        (bind _output_get (set `self.State` "NewEnumerator2"))
        (`Controller.StopMovement` (`self.Ai`)))
      (:`then_1`
        (set `/Game/Blueprints/Character/ABP_Enemy.AnimState` _output_get _anim)
        (set `/Game/Blueprints/Character/ABP_Enemy.bAttackPlay` true _anim)
        (set `self.CurrentTime` (- (`self.DamageDelayTime`) 0.1))))))