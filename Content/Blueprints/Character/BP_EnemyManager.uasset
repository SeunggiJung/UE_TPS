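; BP_EnemyManager is a manager meant to spawn BP_Enemy actors periodically at spawn points, though its spawning logic is currently disconnected.
; On BeginPlay it starts a looping timer and caches all BP_EnemySpawnPoint actors.
; CreateEnemy has an empty body, with unconnected nodes that would spawn at a random point below a population limit.
; GetRandomPosition computes a random horizontal offset from a point's sphere radius but is never called here.
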(event `self.ReceiveBeginPlay`
  (`|ExecutionSequence`
    (:`then_0`
      (bind _returnvalue (`KismetSystemLibrary.K2_SetTimerDelegate` (`|CreateDelegate` :!event `CreateEnemy`) 5.0 true))
      (set `self.HandleTimer` _returnvalue))
    (:`then_1`
      (`KismetArrayLibrary.Array_Clear` (`self.SpawnPoints`))
      (bind _outactors (`GameplayStatics.GetAllActorsOfClass` "/Game/Blueprints/Character/BP_EnemySpawnPoint.BP_EnemySpawnPoint_C"))
      (for _array_element _outactors
        (`KismetArrayLibrary.Array_Add` (`self.SpawnPoints`) _array_element)))))

(fn `CreateEnemy`)

(fn `GetRandomPosition`
  (params (SpawnPoint :type "/Game/Blueprints/Character/BP_EnemySpawnPoint Object Reference"))
  (returns (RnadomLocation :type "Vector Structure"))
  (set `self.SpawnPointLocation` (`self.K2_GetActorLocation` SpawnPoint))
  (set `self.LocalSphereRadius` (`SphereComponent.GetUnscaledSphereRadius` (`/Game/Blueprints/Character/BP_EnemySpawnPoint.Sphere` SpawnPoint)))
  (bind _output_get (set `self.RandomVector` (`KismetMathLibrary.MakeVector` (`KismetMathLibrary.RandomFloatInRange` -1.0 1.0) (`KismetMathLibrary.RandomFloatInRange` -1.0 1.0))))
  (return (+ (* (`KismetMathLibrary.Normal` _output_get) (`KismetMathLibrary.RandomFloatInRange` -1.0 (`self.LocalSphereRadius`))) (`self.SpawnPointLocation`))))

(fn `UserConstructionScript`)