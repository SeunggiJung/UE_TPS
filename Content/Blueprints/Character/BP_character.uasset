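; Player shooter character that switches between a grenade gun spawning BP_Bullet projectiles and a hitscan sniper rifle with a zoomed scope UI.
; Sniper traces from the camera push physics objects and damage BP_Enemy through its FSM; firing plays montage, shake and sound.
; It creates the HUD, handles sprint and health, reports weapon, damage and game-over events through the GameInstance's event dispatcher, and pauses on death.
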(event `EnhancedInput|/Game/Blueprints/Inputs/IA_Fire`
  (params (ActionValue :type Boolean) (ElapsedSeconds :type "Float (double-precision)") (TriggeredSeconds :type "Float (double-precision)") (InputAction :type "InputAction Object Reference" :default "/Game/Blueprints/Inputs/IA_Fire.IA_Fire"))
  (:`Started`
    (`|ExecutionSequence`
      (:`then_0`
        (if (`self.Using Granade Gun`)
          (`|SpawnActorFromClass` "/Game/Blueprints/Character/BP_Bullet.BP_Bullet_C" (`SceneComponent.GetSocketTransform` (`self.Gun Mesh`) "FirePosition" "RTS_World") "Undefined" "MultiplyWithRoot" null null)
          (else
            (`self.SniperHitScan`))))
      (:`then_1`
        (`|PlayMontage` (`self.Mesh`) "/Game/Animations/Fire_Rifle_Ironsights_Montage.Fire_Rifle_Ironsights_Montage"
          (:`then`
            (`PlayerCameraManager.StartCameraShake` :`self` (`GameplayStatics.GetPlayerCameraManager` 0) :`ShakeClass` "/Game/Blueprints/etc/BP_CameraShake.BP_CameraShake_C")
            (`GameplayStatics.PlaySound2D` "/Game/SniperGun/Rifle.Rifle" 1.0 1.0 0.0 null null)))))))

(event `EnhancedInput|/Game/Blueprints/Inputs/IA_Fire`
  (params (ActionValue :type Boolean) (ElapsedSeconds :type "Float (double-precision)") (TriggeredSeconds :type "Float (double-precision)") (InputAction :type "InputAction Object Reference" :default "/Game/Blueprints/Inputs/IA_Fire.IA_Fire"))
  ; Bool형 변수
)

(event `self.ReceiveBeginPlay`
  (`|ExecutionSequence`
    (:`then_0`
      (`self.Initialize`))
    (:`then_1`
      (`self.ChangeGun`))))

(event `EnhancedInput|/Game/Blueprints/Inputs/IA_GrenadeGun`
  (params (ActionValue :type Boolean) (ElapsedSeconds :type "Float (double-precision)") (TriggeredSeconds :type "Float (double-precision)") (InputAction :type "InputAction Object Reference" :default "/Game/Blueprints/Inputs/IA_GrenadeGun.IA_GrenadeGun"))
  ; 총 변경
  (:`Started`
    (set `self.Using Granade Gun` true)
    (`self.ChangeGun`)))

(event `EnhancedInput|/Game/Blueprints/Inputs/IA_SniperMode`
  (params (ActionValue :type Boolean) (ElapsedSeconds :type "Float (double-precision)") (TriggeredSeconds :type "Float (double-precision)") (InputAction :type "InputAction Object Reference" :default "/Game/Blueprints/Inputs/IA_SniperMode.IA_SniperMode"))
  (bind _sniperui (`self.SniperUI`))
  (bind _camera (`self.Camera`))
  (bind _crosshairui (`self.CrosshairUI`))
  ; 스나이퍼 UI
  (:`Triggered`
    (`UserWidget.AddToViewport` _sniperui 0)
    (`CameraComponent.SetFieldOfView` _camera 45.0)
    (`Widget.RemoveFromParent` _crosshairui))
  (:`Completed`
    (`Widget.RemoveFromParent` _sniperui)
    (`CameraComponent.SetFieldOfView` _camera 90.0)
    (`UserWidget.AddToViewport` _crosshairui 0)))

(event `self.ReceiveTick`
  (params (DeltaSeconds :type "Float (single-precision)"))
  (bind _outactors (`GameplayStatics.GetAllActorsOfClass` "/Game/Blueprints/Tutorial/BP_Tutorial.BP_Tutorial_C"))
  (if (`KismetMathLibrary.Conv_IntToBool` (`KismetArrayLibrary.Array_Length` _outactors))
    (set `self.TutorialTarget` (`|GetArrayItem` _outactors))))

(event `EnhancedInput|/Game/Blueprints/Inputs/IA_Sniper`
  (params (ActionValue :type Boolean) (ElapsedSeconds :type "Float (double-precision)") (TriggeredSeconds :type "Float (double-precision)") (InputAction :type "InputAction Object Reference" :default "/Game/Blueprints/Inputs/IA_Sniper.IA_Sniper"))
  ; 총 변경
  (:`Started`
    (set `self.Using Granade Gun` false)
    (`self.ChangeGun`)))

(event `EnhancedInput|/Game/Blueprints/Inputs/IA_Run`
  (params (ActionValue :type Boolean) (ElapsedSeconds :type "Float (double-precision)") (TriggeredSeconds :type "Float (double-precision)") (InputAction :type "InputAction Object Reference" :default "/Game/Blueprints/Inputs/IA_Run.IA_Run"))
  (bind _charactermovement (`self.CharacterMovement`))
  (:`Started`
    (set `CharacterMovementComponent.MaxWalkSpeed` (`self.Runspeed`) _charactermovement))
  (:`Completed`
    (set `CharacterMovementComponent.MaxWalkSpeed` (`self.Walkspeed`) _charactermovement)))

(fn `ChangeGun`
  (bind _using_granade_gun (`self.Using Granade Gun`))
  (`SceneComponent.SetVisibility` (`self.Gun Mesh`) _using_granade_gun false)
  (`SceneComponent.SetVisibility` (`self.Gun Mesh1`) false false)
  (`SceneComponent.SetVisibility` (`self.SniperGun Mesh`) (not _using_granade_gun) false)
  (`/Game/Blueprints/GameConfig/BP_GameEventDispather.OnUsingGrenade` (`self.GameEventDispatcher`) (`self.Using Granade Gun`)))

(fn `Initialize`
  (`|ExecutionSequence`
    (:`then_0`
      (bind _returnvalue (`|CreateWidget` "/Game/Blueprints/UMG/WBP_SniperUI.WBP_SniperUI_C"))
      (set `self.SniperUI` _returnvalue))
    (:`then_1`
      (set `CharacterMovementComponent.MaxWalkSpeed` (`self.Walkspeed`) (`self.CharacterMovement`))
      (set `self.CurrHp` (`self.InitialHp`))
      (bind _asbp_game_instance (cast `/Game/Blueprints/GameConfig/BP_GameInstance` (`GameplayStatics.GetGameInstance`)))
      (bind _output_get (set `self.GameEventDispatcher` (`/Game/Blueprints/GameConfig/BP_GameInstance.GameEventDispatcher` _asbp_game_instance)))
      (`/Game/Blueprints/GameConfig/BP_GameEventDispather.OnDataLoadComplete` _output_get))
    (:`then_2`
      (bind _returnvalue_2 (`|CreateWidget` "/Game/Blueprints/UMG/WBP_Crosshair.WBP_Crosshair_C"))
      (bind _output_get_2 (set `self.CrosshairUI` _returnvalue_2))
      (`UserWidget.AddToViewport` _output_get_2 0))
    (:`then_3`
      (bind _returnvalue_3 (`|CreateWidget` "/Game/Blueprints/UMG/WBP_ScreenUI.WBP_ScreenUI_C"))
      (bind _output_get_3 (set `self.ScreenUI` _returnvalue_3))
      (`UserWidget.AddToViewport` _output_get_3 0))
    (:`then_4`
      (`/Game/Blueprints/GameConfig/BP_GameEventDispather.OnDataLoadComplete` (`self.GameEventDispatcher`)))))

(fn `OnDamageProcess`
  (locals (LocalCenterPosition :type "Vector Structure") (LocalCameraPosition :type "Vector Structure") (LocalEffectFrontDir :type "Vector Structure"))
  (if (> (`self.CurrHp`) 0.0)
    (`|ExecutionSequence`
      (:`then_0`
        (bind _output_get (set `self.CurrHp` (- (`self.CurrHp`) (`self.DamageValue`))))
        (if (<= _output_get 0.0)
          (`self.OnGameOver`)))
      (:`then_1`
        (bind _asbp_game_instance (cast `/Game/Blueprints/GameConfig/BP_GameInstance` (`GameplayStatics.GetGameInstance`)))
        (`/Game/Blueprints/GameConfig/BP_GameEventDispather.OnPlayerDamaged` (`/Game/Blueprints/GameConfig/BP_GameInstance.GameEventDispatcher` _asbp_game_instance) self (`self.DamageValue`)))
      (:`then_2`
        (set `local.LocalCenterPosition` (`SceneComponent.K2_GetComponentLocation` (`self.CapsuleComponent`)))
        (set `local.LocalCameraPosition` (`SceneComponent.K2_GetComponentLocation` (`self.Camera`)))
        (set `local.LocalEffectFrontDir` (0.0 0.0 0.0))
        (`GameplayStatics.SpawnEmitterAtLocation` "/Game/StarterContent/Particles/P_BulletEffect.P_BulletEffect" (+ (`local.LocalCenterPosition`) (* (`KismetMathLibrary.Normal` (- (`local.LocalCameraPosition`) (`local.LocalCenterPosition`))) 50.0) (0.0 0.0 20.0) (* (`KismetMathLibrary.RandomUnitVector`) (`KismetMathLibrary.RandomFloatInRange` 5.0 35.0))))))))

(fn `OnGameOver`
  (bind _returnvalue (`GameplayStatics.GetPlayerController` 0))
  (`GameplayStatics.SetGamePaused` true)
  (bind _returnvalue_2 (`|CreateWidget` "/Game/Blueprints/UMG/WBP_GameOverUI.WBP_GameOverUI_C" _returnvalue))
  (`UserWidget.AddToViewport` _returnvalue_2 0)
  (set `PlayerController.bShowMouseCursor` true _returnvalue)
  (`/Game/Blueprints/GameConfig/BP_GameEventDispather.OnGameOver` (`self.GameEventDispatcher`)))

(fn `SniperHitScan`
  (bind _camera (`self.Camera`))
  (bind _returnvalue (`SceneComponent.K2_GetComponentLocation` _camera))
  (set `self.StartPos` _returnvalue)
  (set `self.EndPos` (+ _returnvalue (* (`SceneComponent.GetForwardVector` _camera) (`self.TraceDistance`))))
  (bind (_outhit _returnvalue_2) (`KismetSystemLibrary.LineTraceSingle` (`self.StartPos`) (`self.EndPos`) "TraceTypeQuery1"))
  (`|ExecutionSequence`
    (:`then_0`
      (bind (_bblockinghit _binitialoverlap _time _distance _location _impactpoint _normal _impactnormal _physmat _hitactor _hitcomponent) (`GameplayStatics.BreakHitResult` _outhit))
      (if _bblockinghit
        (`|ExecutionSequence`
          (:`then_0`
            (`GameplayStatics.SpawnEmitterAtLocation` "/Game/StarterContent/Particles/P_BulletEffect.P_BulletEffect" _location))
          (:`then_1`
            (if (and (`KismetSystemLibrary.IsValid` _hitcomponent) (`SceneComponent.IsSimulatingPhysics` _hitcomponent "None"))
              (bind _output_get (set `self.NormalLine` (- (`self.EndPos`) (`self.StartPos`))))
              (`PrimitiveComponent.AddForceAtLocation` _hitcomponent (* _output_get 1000.0) _returnvalue "None"))))))
    (:`then_1`
      (if _returnvalue_2
        (bind _asbp_enemy (cast `/Game/Blueprints/Character/BP_Enemy` _hitactor))
        (`/Game/Blueprints/Character/BP_EnemyFSM.OnDamageProcess` (`/Game/Blueprints/Character/BP_Enemy.Fsm(FSM)` _asbp_enemy))))))

(fn `UserConstructionScript`)